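; Player pawn for the card game, which builds its deck from the game instance and routes damage to its StatsComponent.
; TurnComponent events drive turn effects, energy reset and interaction, while activated cards spend energy and interaction follows remaining energy.
; Ending a turn, winning or losing staggers hand discards by index, using a timer to wait for an empty hand before TryEndTurn.
; An interface function exposes the TurnComponent.
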(event OnStartTurn(TurnComponent)
  (Class|CZPlayerPawn|StartTurn)
  (Default|ResetEnergy (Variables|Default|GetStatsComponent))
  (Class|CZPlayerPawn|EnableInteract true))

(event OnWin(TurnComponent)
  (Class|CZPlayerPawn|EnableInteract false)
  (for _array_element (Class|CZPlayerPawn|GetHand)
    (bind _asbp_card_parent (Utilities|Casting|CastToBP_CardParent _array_element))
    (Default|DelayDiscard _asbp_card_parent (* (Class|CZCard|GetHandIndex _array_element) 0.25)))
  (CallFunction|CheckforEndTurn))

(event OnEnergyChanged(StatsComponent)
  (params (Energy :type Integer) (MaxEnergy :type Integer))
  (Class|CZPlayerPawn|EnableInteract (> Energy 0.0)))

(event OnPrepareEndTurn(TurnComponent)
  (Class|CZEffectsComponent|TurnEnd (Variables|Default|GetEffectComponent))
  (Class|CZPlayerPawn|EnableInteract false)
  (for _array_element (Class|CZPlayerPawn|GetHand)
    (bind _asbp_card_parent (Utilities|Casting|CastToBP_CardParent _array_element))
    (Default|DelayDiscard _asbp_card_parent (* (Class|CZCard|GetHandIndex _array_element) 0.25)))
  (CallFunction|CheckforEndTurn))

(event OnLose(TurnComponent)
  (params (Component :type BP%20Turn%20Component%20Object%20Reference))
  (Class|CZPlayerPawn|EnableInteract false)
  (for _array_element (Class|CZPlayerPawn|GetHand)
    (bind _asbp_card_parent (Utilities|Casting|CastToBP_CardParent _array_element))
    (Default|DelayDiscard _asbp_card_parent (* (Class|CZCard|GetHandIndex _array_element) 0.25)))
  (CallFunction|CheckforEndTurn))

(event OnPrepareStartTurn(TurnComponent)
  (Class|CZEffectsComponent|TurnStart (Variables|Default|GetEffectComponent)))

(event Game|Damage|EventAnyDamage
  (params (Damage :type Float%20%28single-precision%29) (DamageType :type Damage%20Type%20Object%20Reference) (InstigatedBy :type Controller%20Object%20Reference) (DamageCauser :type Actor%20Object%20Reference))
  (Default|ApplyDamage (Variables|Default|GetStatsComponent) (Math|Float|Truncate Damage)))

(event EventOnCardActivated
  (params (Cost :type Integer))
  (Default|UseEnergy (Variables|Default|GetStatsComponent) Cost))

(event EventBeginPlay
  (Class|CZPlayerPawn|CreateDeck (Variables|/Game/MyContent/Core/BP_GameInstance.BP_GameInstance_C|GetPlayerDeck (CallFunction|GetCardGameInstance))))

(fn ConstructionScript)

(fn CheckforEndTurn
  (if (Utilities|Array|IsNotEmpty (Class|CZPlayerPawn|GetHand))
    (Utilities|Time|SetTimerbyEvent (EventDispatchers|CreateEvent :!event CheckforEndTurn) 0.2)
    (else
      (Default|TryEndTurn (Variables|Default|GetTurnComponent))
      (Variables|Default|SetDiscardCounter 0))))

(fn BIBMGetTurnComponent
  (return (Variables|Default|GetTurnComponent)))