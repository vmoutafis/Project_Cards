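; BP_CardPlayerPawn is the player pawn in a card game with turn-based play.
; On BeginPlay it builds its deck from the PlayerDeck stored in the card game instance.
; Its turn component's events start the turn and enable interaction, then disable interaction and clear the hand when the turn ends.
; An interface function exposes that turn component to other code.
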(event OnStartTurn(AC_TurnComponent)
  (Class|CZPlayerPawn|StartTurn)
  (Class|CZPlayerPawn|EnableInteract true))

(event OnEndTurn(AC_TurnComponent)
  (Class|CZPlayerPawn|EnableInteract false)
  (Class|CZPlayerPawn|ClearHand))

(event EventBeginPlay
  (Class|CZPlayerPawn|CreateDeck (Variables|/Game/MyContent/Core/BP_GameInstance.BP_GameInstance_C|GetPlayerDeck (CallFunction|GetCardGameInstance))))

(fn ConstructionScript)

(fn BIBMGetTurnComponent
  (return (Variables|Default|GetAC_TurnComponent)))