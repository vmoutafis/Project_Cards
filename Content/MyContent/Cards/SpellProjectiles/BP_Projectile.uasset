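; Card spell projectile that flies toward its facing direction and damages an assigned target.
; ActivateSpell stores the target and launches the projectile by setting its movement velocity from forward vector and speed.
; The sphere overlap destroys the projectile only on contact with that target.
; Damage, using the scaled spell value, is applied in the destroyed handler rather than on overlap, so any destruction damages the target.
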(event OnComponentBeginOverlap(Sphere)
  (params (OverlappedComponent :type Primitive%20Component%20Object%20Reference) (OtherActor :type Actor%20Object%20Reference) (OtherComp :type Primitive%20Component%20Object%20Reference) (OtherBodyIndex :type Integer) (bFromSweep :type Boolean) (SweepResult :type Hit%20Result%20Structure%20%28by%20ref%29))
  (if (== OtherActor (Variables|Default|GetTarget))
    (Actor|DestroyActor)))

(event EventBeginPlay
  (Game|BindEventtoOnDestroyed (EventDispatchers|CreateEvent :!event OnProjectileDestroyed)))

(fn ConstructionScript)

(fn OnProjectileDestroyed
  (params (DestroyedActor :type Actor%20Object%20Reference))
  (Game|Damage|ApplyDamage (Variables|Default|GetTarget) (CallFunction|GetValueScaled) 0 (Components|GetOwner) (Variables|Default|GetDamageTypeClass)))

(fn ActivateSpell
  (params (Target :type Actor%20Object%20Reference))
  (Variables|Default|SetTarget Target)
  (CallFunction|LaunchProjectile))

(fn LaunchProjectile
  (Variables|/Script/Engine.MovementComponent|SetVelocity (Variables|Default|GetProjectileMovement) (* (Transformation|GetActorForwardVector) (Variables|Default|GetSpeed))))