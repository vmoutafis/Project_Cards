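; Spell card that, when activated, turns into a spawned spell aimed at the hit location.
; Activation stores the hit actor and location, then a timeline shrinks the card to zero scale.
; When the shrink finishes, it spawns SpellClass at the card's position, passing Value, owner and current scale.
; It then calls ActivateSpell with the hit actor before running the parent's completion logic.
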(event Custom|LerpShrink
  (Components|Timeline|SetPlayRate (Variables|Default|GetTL_ShrinkCard) (/ 1.0 0.25))
  (Variables|Default|SetLerpStartScale (Transformation|GetActorScale3D))
  (bind _alpha (Timeline|TL_ShrinkCard PlayFromStart)
    (:Update
      (Transformation|SetActorScale3D (Math|Vector|Lerp(Vector) (Variables|Default|GetLerpStartScale) "0, 0, 0" _alpha)))
    (:Finished
      (CallFunction|OnCardActivatedComplete))))

(fn ConstructionScript
  (|CallParentFunction))

(fn OnCardActivated
  (params (HitActor :type Actor%20Object%20Reference) (HitLocation :type Vector :default "0, 0, 0"))
  (Variables|Default|SetHitActor HitActor)
  (Variables|Default|SetHitLocation HitLocation)
  (CallFunction|LerpShrink))

(fn OnCardActivatedComplete
  (bind _returnvalue (Transformation|GetActorTransform))
  (bind _returnvalue_2 (Game|SpawnActorfromClass (Variables|Spell|GetSpellClass) (Math|Transform|MakeTransform (.location _returnvalue) (Math|Rotator|FindLookatRotation (.location _returnvalue) (Variables|Default|GetHitLocation)) (.scale _returnvalue)) "Undefined" "MultiplyWithRoot" (Components|GetOwner) (Variables|Spell|GetValue) 0))
  (Default|ActivateSpell _returnvalue_2 (Variables|Default|GetHitActor))
  (|CallParentFunction))