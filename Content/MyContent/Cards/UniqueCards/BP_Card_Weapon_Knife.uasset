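; Knife weapon card that inflicts a turn-based bleed on the actors it damages.
; When damage is applied, it looks for the target's BP_EffectComponent and, if present, adds a short Bleed damage-over-time effect with itself as the causer.
; The bleed damage doubles when the gameplay tags include Critical.
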(fn ConstructionScript
  (|CallParentFunction))

(fn OnDamageApplied
  (params (DamagedActor :type Actor%20Object%20Reference))
  (bind _returnvalue (Actor|GetComponentbyClass DamagedActor "/Game/MyContent/Effects/BP_EffectComponent.BP_EffectComponent_C"))
  (bind _damageovertime (Variables|Default|GetDamageOverTime))
  (Utilities|IsValid _returnvalue
    (:Is%20Valid
      (Default|AddDoTEffect _returnvalue "/Game/MyContent/Effects/UniqueEffects/BP_Effect_TD_DoT_Bleed.BP_Effect_TD_DoT_Bleed_C" 2 (Math|Float|SelectFloat (* _damageovertime 2.0) _damageovertime (GameplayTags|HasTag (Variables|Default|GetGameplayTags) "(TagName=\"Critical\")")) self))))