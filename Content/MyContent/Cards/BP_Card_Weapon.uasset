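; BP_Card_Weapon is a card that, when activated on a target, flies to the hit location and damages the hit actor.
; A timeline timed by FlyToTargetSpeed lerps location and turns pitch and yaw toward the hit, leaving roll free while RotatingMovement runs.
; On arrival it applies damage scaled by a game instance attribute, then calls the parent completion.
; Resetting the card stops the rotating movement.
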(event Custom|LerpToHitActor
  (bind _returnvalue (Transformation|GetActorLocation))
  (bind _hitlocation (Variables|Default|GetHitLocation))
  (bind _returnvalue_2 (Math|Rotator|FindLookatRotation _returnvalue _hitlocation))
  (Variables|Default|GetHitActor
    (:then
      (Components|Activation|Activate (Variables|Default|GetRotatingMovement) false)
      (Components|Timeline|SetPlayRate (Variables|Default|GetTL_LerpToHitActor) (/ 1.0 (Variables|Weapon|GetFlyToTargetSpeed)))
      (Variables|Default|SetStartLerpTrans (Transformation|GetActorTransform))
      (Variables|Default|SetHitLookAtRotation (Math|Rotator|MakeRotator (.roll _returnvalue_2) (+ (.pitch _returnvalue_2) -9e+01) (.yaw _returnvalue_2)))
      (bind (_direction _alpha _rotalpha) (Timeline|TL_LerpToHitActor PlayFromStart)
        (:Update
          (Utilities|FlowControl|Sequence
            (:then_0
              (Transformation|SetActorLocation (Math|Vector|Lerp(Vector) (.location (Variables|Default|GetStartLerpTrans)) (Variables|Default|GetHitLocation) _alpha) false false))
            (:then_1
              (Transformation|SetActorRotation (Math|Rotator|MakeRotator (.roll (Transformation|GetActorRotation)) (.pitch (Math|Rotator|Lerp(Rotator) (.rotation (Variables|Default|GetStartLerpTrans)) (Variables|Default|GetHitLookAtRotation) _rotalpha true)) (.yaw (Math|Rotator|Lerp(Rotator) (.rotation (Variables|Default|GetStartLerpTrans)) (Variables|Default|GetHitLookAtRotation) _rotalpha true)))))))
        (:Finished
          (CallFunction|OnCardActivatedComplete))))
    (:else)))

(fn ConstructionScript
  (|CallParentFunction))

(fn OnCardActivated
  (params (HitActor :type Actor%20Object%20Reference) (HitLocation :type Vector :default "0, 0, 0"))
  (Variables|Default|SetHitActor HitActor)
  (Variables|Default|SetHitLocation HitLocation)
  (CallFunction|LerptoHitActor))

(fn OnCardActivatedComplete
  (Game|Damage|ApplyDamage (Variables|Default|GetHitActor) (* (Variables|Weapon|GetDamage) (Default|GetAttribute (CallFunction|GetCardGameInstance) "NewEnumerator0")) 0 (Game|Player|GetPlayerPawn 0) (Variables|Weapon|GetDamageTypeClass))
  (|CallParentFunction))

(fn ResetCard
  (params (Location :type Vector :default "0, 0, 0"))
  (|CallParentFunction Location)
  (Components|Activation|Deactivate (Variables|Default|GetRotatingMovement)))