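; Melee card Blueprint that spins and lunges the card at its hit location to deliver its effects.
; On activation it starts a fast constant mesh rotation, then a short timeline lerps the card from its current location to the hit point.
; When the timeline finishes it completes activation, which stops the spin, applies effects and starts discarding the card.
; A card reset also stops the spin.
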(event EventOnActivationComplete
  (CallFunction|StopConstantMeshRotate true)
  (Class|CZCard|ApplyEffects)
  (Class|CZCard|StartDiscard true))

(event EventOnCardReset
  (CallFunction|StopConstantMeshRotate true))

(event EventOnCardActivated
  (CallFunction|ConstantMeshRotate "0.000000,3000.000000,0.000000" false true)
  (Variables|Default|SetMeleeStartLocation (.location (Class|CZCard|GetCurrentTransform)))
  (Components|Timeline|SetPlayRate (Variables|Default|GetTL_LerpToTarget) (/ 1.0 0.25))
  (bind _alpha (Timeline|TL_LerpToTarget PlayFromStart)
    (:Update
      (Class|CZCard|TransformCardOffset (Math|Transform|MakeTransform (Math|Vector|Lerp(Vector) (Variables|Default|GetMeleeStartLocation) (Class|CZCard|GetHitLocation) _alpha) "-90.000000,0.000000,0.000000" "1.000000,1.000000,1.000000") 5e+01))
    (:Finished
      (Class|CZCard|CompleteActivation))))

(fn ConstructionScript
  (|CallParentFunction))