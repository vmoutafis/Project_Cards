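; BP_Card_Ranged is a card that fires a projectile at the actor and location it was activated on.
; On activation it spawns a disperse Niagara effect and a projectile at its own position, then launches it with the owner as source and the card's effect objects as payload.
; It completes activation right after launch, without waiting for impact, and starts discarding once activation completes.
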(event EventOnActivationComplete
  (Class|CZCard|StartDiscard true))

(event EventOnCardActivated
  (params (actorHit :type Actor%20Object%20Reference) (locationHit :type Vector :default "0, 0, 0"))
  (Niagara|SpawnSystematLocation (Variables|Default|GetCardDisperseEffect) (Transformation|GetActorLocation))
  (bind _returnvalue (Game|SpawnActorfromClass (Variables|Card|GetProjectileClass) (Math|Transform|MakeTransform (Transformation|GetActorLocation) "0, 0, 0" "1.000000,1.000000,1.000000") "AlwaysSpawn" "MultiplyWithRoot" 0 0))
  (Class|CZProjectile|LaunchProjectile _returnvalue (Components|GetOwner) actorHit locationHit (Variables|Default|GetCardEffectsObjects) 2e+03)
  (Class|CZCard|CompleteActivation))

(fn ConstructionScript
  (|CallParentFunction))