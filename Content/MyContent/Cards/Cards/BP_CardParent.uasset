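; BP_CardParent is the base card Blueprint, handling the name text, mesh spin and discard sequence shared by cards.
; Activation completion or a timed delay starts a discard, whose activation spins the mesh while a timeline lifts and shrinks it before completing the discard.
; Construction writes CardName to the text render and points RotatingMovement at the mesh; spin helpers toggle that component alongside the mesh lerp.
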(event Custom|DelayDiscard
  (params (Time :type Float%20%28double-precision%29))
  (Utilities|FlowControl|Delay Time)
  (Class|CZCard|StartDiscard false))

(event EventOnDiscardActivated
  (Class|CZCard|ChangeLerpType "CLT_ActorOnly")
  (CallFunction|ConstantMeshRotate "0.000000,0.000000,1000.000000" false true)
  (bind (_direction _alpha _scalealpha) (Timeline|TL_DiscardLift PlayFromStart)
    (:Update
      (Utilities|FlowControl|Sequence
        (:then_0
          (Transformation|SetRelativeLocation (Variables|Character|GetMesh) (Math|Vector|MakeVector 0.0 0.0 (Math|Float|Lerp 0.0 25.0 _alpha)) false false))
        (:then_1
          (Transformation|SetRelativeScale3D (Variables|Character|GetMesh) (Math|Vector|Lerp(Vector) "1.000000,1.000000,1.000000" "0, 0, 0" _scalealpha)))))
    (:Finished
      (Class|CZCard|CompleteDiscard))))

(event EventOnActivationComplete
  (Class|CZCard|StartDiscard false))

(fn ConstructionScript
  (CallFunction|UpdateCardNameText)
  (Components|Movement|SetUpdatedComponent (Variables|Default|GetRotatingMovement) (Variables|Character|GetMesh)))

(fn UpdateCardNameText
  (Rendering|Components|TextRender|SetText (Variables|Default|GetTextRender) (Utilities|Text|ToText(String) (Variables|Default|GetCardName))))

(fn ConstantMeshRotate
  (params (Speed :type Rotator) (bReset :type Boolean) (bStopMeshLerp :type Boolean))
  (Components|Activation|Activate (Variables|Default|GetRotatingMovement) bReset)
  (Variables|/Script/Engine.RotatingMovementComponent|SetRotationRate (Variables|Default|GetRotatingMovement) Speed)
  (Class|CZCard|IgnoreMeshLerp bStopMeshLerp))

(fn StopConstantMeshRotate
  (params (bAllowMeshLerp :type Boolean))
  (Variables|/Script/Engine.RotatingMovementComponent|SetRotationRate (Variables|Default|GetRotatingMovement) "0, 0, 0")
  (Components|Activation|Deactivate (Variables|Default|GetRotatingMovement))
  (Class|CZCard|IgnoreMeshLerp (not bAllowMeshLerp)))