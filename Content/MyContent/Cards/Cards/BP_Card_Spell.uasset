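; Spell card Blueprint that plays an activation animation, applies its effects and is then discarded.
; On activation, a short timeline lerps the card from its captured transform upward while turning it half around in yaw and shrinking it to zero scale.
; The timeline's end calls CompleteActivation, and the activation-complete event applies effects and starts the discard.
; Card reset stops the constant mesh rotation.
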(event EventOnActivationComplete
  (Class|CZCard|ApplyEffects)
  (Class|CZCard|StartDiscard true))

(event EventOnCardReset
  (CallFunction|StopConstantMeshRotate true))

(event EventOnCardActivated
  (Components|Timeline|SetPlayRate (Variables|Default|GetTL_AnimateActivate) (/ 1.0 0.2))
  (Variables|Default|SetSpellActivateLocation (Class|CZCard|GetCurrentTransform))
  (bind _alpha (Timeline|TL_AnimateActivate PlayFromStart)
    (:Update
      (Class|CZCard|TransformCardActor (Math|Transform|MakeTransform (.location (Math|Transform|Lerp(Transform) (Variables|Default|GetSpellActivateLocation) (Math|Transform|MakeTransform (+ (.location (Variables|Default|GetSpellActivateLocation)) "0.000000,0.000000,100.000000") (Math|Rotator|MakeRotator (.roll (.rotation (Variables|Default|GetSpellActivateLocation))) (.pitch (.rotation (Variables|Default|GetSpellActivateLocation))) (Math|Rotator|NormalizeAxis (+ (.yaw (.rotation (Variables|Default|GetSpellActivateLocation))) 1.8e+02))) "0.000000,0.000000,0.000000") _alpha)) (.rotation (Math|Transform|Lerp(Transform) (Variables|Default|GetSpellActivateLocation) (Math|Transform|MakeTransform (+ (.location (Variables|Default|GetSpellActivateLocation)) "0.000000,0.000000,100.000000") (Math|Rotator|MakeRotator (.roll (.rotation (Variables|Default|GetSpellActivateLocation))) (.pitch (.rotation (Variables|Default|GetSpellActivateLocation))) (Math|Rotator|NormalizeAxis (+ (.yaw (.rotation (Variables|Default|GetSpellActivateLocation))) 1.8e+02))) "0.000000,0.000000,0.000000") _alpha)) (.scale (Math|Transform|Lerp(Transform) (Variables|Default|GetSpellActivateLocation) (Math|Transform|MakeTransform (+ (.location (Variables|Default|GetSpellActivateLocation)) "0.000000,0.000000,100.000000") (Math|Rotator|MakeRotator (.roll (.rotation (Variables|Default|GetSpellActivateLocation))) (.pitch (.rotation (Variables|Default|GetSpellActivateLocation))) (Math|Rotator|NormalizeAxis (+ (.yaw (.rotation (Variables|Default|GetSpellActivateLocation))) 1.8e+02))) "0.000000,0.000000,0.000000") _alpha))) 5e+01))
    (:Finished
      (Class|CZCard|CompleteActivation))))

(fn ConstructionScript
  (|CallParentFunction))