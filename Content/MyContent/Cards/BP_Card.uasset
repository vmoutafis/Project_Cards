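; BP_Card is a playing card actor in the hand that can be highlighted, dragged, activated and reset, with an energy cost shown on a widget.
; Hover, click or touch highlights it by shifting the mesh and cancelling its rotation, while click or touch also calls DragCard on BP_PlayerPawn.
; Tick interpolates actor and mesh toward target transforms, faster while dragging.
; Dispatchers report highlight changes and activation completion with the hand index.
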(event EventBeginPlay
  (CallFunction|UpdateCostText))

(event EventTick
  (params (DeltaSeconds :type Float%20%28single-precision%29))
  (CallFunction|HandleActorInterp)
  (CallFunction|HandleMeshInterp))

(event EventActorOnInputTouchBegin
  (params (FingerIndex :type ETouchIndex%20Enum :default "Touch1"))
  (bind _asbp_player_pawn (Utilities|Casting|CastToBP_PlayerPawn (Game|Player|GetPlayerPawn 0)))
  (if (and (not (Utilities|IsValid (Variables|/Game/MyContent/Player/BP_PlayerPawn.BP_PlayerPawn_C|GetDraggingCard _asbp_player_pawn))) (not (Variables|Default|GetbDragging)))
    (CallFunction|HighlightCard)
    (bind _asbp_player_pawn_2 (Utilities|Casting|CastToBP_PlayerPawn (Game|Player|GetPlayerPawn 0)))
    (Default|DragCard _asbp_player_pawn_2)))

(event MouseInput|EventActorOnClicked
  (params (ButtonPressed :type Key%20Structure :default "None"))
  (bind _asbp_player_pawn (Utilities|Casting|CastToBP_PlayerPawn (Game|Player|GetPlayerPawn 0)))
  (if (and (not (Utilities|IsValid (Variables|/Game/MyContent/Player/BP_PlayerPawn.BP_PlayerPawn_C|GetDraggingCard _asbp_player_pawn))) (not (Variables|Default|GetbDragging)))
    (CallFunction|HighlightCard)
    (bind _asbp_player_pawn_2 (Utilities|Casting|CastToBP_PlayerPawn (Game|Player|GetPlayerPawn 0)))
    (Default|DragCard _asbp_player_pawn_2)))

(event MouseInput|EventActorBeginCursorOver
  (bind _asbp_player_pawn (Utilities|Casting|CastToBP_PlayerPawn (Game|Player|GetPlayerPawn 0)))
  (if (and (not (Utilities|IsValid (Variables|/Game/MyContent/Player/BP_PlayerPawn.BP_PlayerPawn_C|GetDraggingCard _asbp_player_pawn))) (not (Variables|Default|GetbDragging)))
    (CallFunction|HighlightCard)))

(event MouseInput|EventActorEndCursorOver
  (if (not (Variables|Default|GetbDragging))
    (CallFunction|UnHighlightCard)))

(fn ConstructionScript
  (bind _output_get (Variables|Default|SetMeshTransform (Transformation|GetRelativeTransform (Variables|Default|GetMesh))))
  (Variables|Default|SetDeafultMeshTransform _output_get))

(fn SetCardTransform
  (params (CardTransform :type Transform))
  (if (not (Variables|Default|GetbDragging))
    (bind _output_get (Variables|Default|SetCardTransform CardTransform))
    (Variables|Default|SetDragTransform (Math|Transform|MakeTransform (.location _output_get) "0, 0, 0" (.scale _output_get)))
    (else
      (Variables|Default|SetDragTransform CardTransform))))

(fn HighlightCard
  (bind _deafultmeshtransform (Variables|Default|GetDeafultMeshTransform))
  (if (and (not (Variables|Default|GetbHighlighted)) (not (Variables|Default|GetbCardActivated)))
    (Variables|Default|SetbHighlighted true)
    (Variables|Default|SetMeshTransform (Math|Transform|MakeTransform "-50.000000,0.000000,50.000000" (.rotation _deafultmeshtransform) (.scale _deafultmeshtransform)))
    (CallFunction|SetOffsetTransform "0, 0, 0" (Class|KismetMathLibrary|NegateRotator (.rotation (Variables|Default|GetCardTransform))) "0, 0, 0")
    (Default|CallOnHighlight self (Variables|Default|GetHandIndex))))

(fn UnHighlightCard
  (if (and (Variables|Default|GetbHighlighted) (not (Variables|Default|GetbCardActivated)))
    (Variables|Default|SetbHighlighted false)
    (CallFunction|ResetMeshTransforms)
    (CallFunction|SetOffsetTransform "0, 0, 0" "0, 0, 0" "0, 0, 0")
    (Default|CallOnUnHighlight self (Variables|Default|GetHandIndex))))

(fn OnMoveEnd)

(fn OnMoveStart)

(fn StopMoving
  (Utilities|FlowControl|Sequence
    (:then_0
      (if (not (Variables|Default|GetbCardDrawn))
        (Variables|Default|SetbCardDrawn true)))
    (:then_1
      (if (Variables|Default|GetbMoving)
        (Variables|Default|SetbMoving false)
        (if (not (Variables|Default|GetbCardActivated))
          (Transformation|SetActorTransform (Math|Transform|SelectTransform (Variables|Default|GetDragTransform) (CallFunction|TrueTransform) (Variables|Default|GetbDragging)))
          (CallFunction|OnMoveEnd))))))

(fn StartMoving
  (if (and (not (Variables|Default|GetbMoving)) (not (Variables|Default|GetbCardActivated)))
    (Variables|Default|SetbMoving true)
    (CallFunction|OnMoveStart)))

(fn SetHandIndex
  (params (Index :type Integer))
  (Variables|Default|SetHandIndex Index))

(fn SetOffsetTransform
  (params (Location :type Vector) (Rotation :type Rotator) (Scale :type Vector))
  (Variables|Default|SetOffsetTransform (Math|Transform|MakeTransform Location Rotation Scale)))

(fn CardIsinPosition
  (return (Class|KismetMathLibrary|NearlyEqualTransformTransform (Math|Transform|SelectTransform (Variables|Default|GetDragTransform) (CallFunction|TrueTransform) (Variables|Default|GetbDragging)) (Transformation|GetActorTransform) 0.01 0.01 0.01)))

(fn TrueTransform
  (bind _cardtransform (Variables|Default|GetCardTransform))
  (bind _offsettransform (Variables|Default|GetOffsetTransform))
  (return (Math|Transform|MakeTransform (+ (.location _cardtransform) (.location _offsettransform)) (Math|Rotator|MakeRotator (+ (.roll (.rotation _cardtransform)) (.roll (.rotation _offsettransform))) (+ (.pitch (.rotation _cardtransform)) (.pitch (.rotation _offsettransform))) (+ (.yaw (.rotation _cardtransform)) (.yaw (.rotation _offsettransform)))) (+ (.scale _cardtransform) (.scale _offsettransform)))))

(fn EnableMovement
  (params (Enable :type Boolean))
  (Variables|Default|SetbCanMove Enable))

(fn DragCard
  (params (Location :type Vector))
  (bind (_x _y _z) (Math|Vector|BreakVector Location))
  (bind _cardtransform (Variables|Default|GetCardTransform))
  (if (not (Variables|Default|GetbCardActivated))
    (Utilities|FlowControl|Sequence
      (:then_0
        (if (not (Variables|Default|GetbDragging))
          (Variables|Default|SetbDragging true)
          (CallFunction|UnHighlightCard)))
      (:then_1
        (CallFunction|SetCardTransform (Math|Transform|MakeTransform (Math|Vector|MakeVector (+ (.x (.location _cardtransform)) -1e+01) _y _z) "0, 0, 0" (.scale _cardtransform)))
        (CallFunction|SetOffsetTransform "0, 0, 0" "0, 0, 0" "0, 0, 0")))))

(fn EndDrag
  (Variables|Default|SetbDragging false))

(fn ActivateCard
  (params (HitActor :type Actor%20Object%20Reference) (HitLocation :type Vector))
  (if (not (Variables|Default|GetbCardActivated))
    (Variables|Default|SetbCardActivated true)
    (CallFunction|OnCardActivated HitActor HitLocation)))

(fn OnCardActivated
  (params (HitActor :type Actor%20Object%20Reference) (HitLocation :type Vector))
  (CallFunction|OnCardActivatedComplete))

(fn ResetCard
  (params (Location :type Vector))
  (Transformation|SetActorTransform (Math|Transform|MakeTransform Location "0, 0, 0" "1.000000,1.000000,1.000000"))
  (Variables|Default|SetbMoving false)
  (Variables|Default|SetbCardActivated false)
  (Variables|Default|SetbDragging false)
  (Variables|Default|SetbCardDrawn false)
  (Variables|Default|SetHandIndex 0)
  (Variables|Default|SetbHighlighted false)
  (CallFunction|SetCardTransform (Transformation|GetActorTransform))
  (CallFunction|SetOffsetTransform "0, 0, 0" "0, 0, 0" "0, 0, 0")
  (CallFunction|ResetMeshTransforms))

(fn OnCardActivatedComplete
  (Default|CallOnCardActivateComplete self (Variables|Default|GetHandIndex)))

(fn UpdateCostText
  (bind _asbp_uw_card_text (Utilities|Casting|CastToBP_UW_Card_Text (UserInterface|GetWidget (Variables|Default|GetCostWidgetComponent))))
  (Default|SetText _asbp_uw_card_text (Utilities|Text|ToText(Integer) (Variables|Card|GetEnergyCost))))

(fn HandleActorInterp
  (if (Math|Boolean|ANDBoolean (not (CallFunction|CardIsinPosition)) (Variables|Default|GetbCanMove) (not (Variables|Default|GetbCardActivated)))
    (Utilities|FlowControl|Sequence
      (:then_0
        (CallFunction|StartMoving))
      (:then_1
        (Transformation|SetActorTransform (Class|KismetMathLibrary|TInterpto (Transformation|GetActorTransform) (Math|Transform|SelectTransform (Variables|Default|GetDragTransform) (CallFunction|TrueTransform) (Variables|Default|GetbDragging)) (Utilities|Time|GetWorldDeltaSeconds) (Math|Float|SelectFloat 25.0 1e+01 (Variables|Default|GetbDragging))))))
    (else
      (CallFunction|StopMoving))))

(fn HandleMeshInterp
  (if (Math|Boolean|ANDBoolean (not (Class|KismetMathLibrary|NearlyEqualTransformTransform (Transformation|GetRelativeTransform (Variables|Default|GetMesh)) (Variables|Default|GetMeshTransform) 0.01 0.01 0.01)) (Variables|Default|GetbCanMove) (not (Variables|Default|GetbCardActivated)))
    (Transformation|SetRelativeTransform (Variables|Default|GetMesh) (Class|KismetMathLibrary|TInterpto (Transformation|GetRelativeTransform (Variables|Default|GetMesh)) (Variables|Default|GetMeshTransform) (Utilities|Time|GetWorldDeltaSeconds) 1e+01) false false)))

(fn ResetMeshTransforms
  (Variables|Default|SetMeshTransform (Variables|Default|GetDeafultMeshTransform)))