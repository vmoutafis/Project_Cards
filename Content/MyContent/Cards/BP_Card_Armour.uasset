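; Card actor that grants armour to the owning player pawn when activated.
; On activation it starts its rotating movement and shrinks to zero scale over a short timeline.
; When the shrink finishes it adds its Armour value to the owner via BP_PlayerPawn, stops rotating and runs the parent completion logic.
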(event Custom|LerpShrink
  (Components|Timeline|SetPlayRate (Variables|Default|GetTL_ShrinkCard) (/ 1.0 0.5))
  (Variables|Default|SetLerpStartScale (Transformation|GetActorScale3D))
  (bind _alpha (Timeline|TL_ShrinkCard PlayFromStart)
    (:Update
      (Transformation|SetActorScale3D (Math|Vector|Lerp(Vector) (Variables|Default|GetLerpStartScale) "0, 0, 0" _alpha)))
    (:Finished
      (CallFunction|OnCardActivatedComplete))))

(fn ConstructionScript
  (|CallParentFunction))

(fn OnCardActivated
  (params (HitActor :type Actor%20Object%20Reference) (HitLocation :type Vector :default "0, 0, 0"))
  (CallFunction|LerpShrink)
  (Components|Activation|Activate (Variables|Default|GetRotatingMovement) false))

(fn OnCardActivatedComplete
  (CallFunction|AddArmour)
  (Components|Activation|Deactivate (Variables|Default|GetRotatingMovement))
  (|CallParentFunction))

(fn AddArmour
  (bind _asbp_player_pawn (Utilities|Casting|CastToBP_PlayerPawn (Components|GetOwner)))
  (Default|AddArmour _asbp_player_pawn (Variables|Armour|GetArmour)))