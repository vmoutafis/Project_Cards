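; BP_Effect is a base Blueprint for effects that an owner applies to an affected actor.
; ActivateEffect stores and validates both actors, then runs the empty ApplyEffect hook and immediately calls EndEffect.
; EndEffect runs the empty OnEffectEnded hook and broadcasts EffectCompleted with itself.
; A helper deals point damage to the affected actor, crediting the owner as causer, with a hit direction opposite the target's forward vector.
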(fn ActivateEffect
  (params (EffectedActor :type Actor%20Object%20Reference) (EffectOwner :type Actor%20Object%20Reference))
  (bind _output_get (Variables|Default|SetEffectedActor EffectedActor))
  (Utilities|IsValid _output_get
    (:Is%20Valid
      (bind _output_get_2 (Variables|Default|SetEffectOwner EffectOwner))
      (Utilities|IsValid _output_get_2
        (:Is%20Valid
          (CallFunction|OnEffectActivated))))))

(fn OnEffectActivated
  (CallFunction|ApplyEffect)
  (CallFunction|EndEffect))

(fn ApplyEffect)

(fn EndEffect
  (CallFunction|OnEffectEnded)
  (Default|CallEffectCompleted self))

(fn ApplyDamagetoEffected
  (params (Damage :type Float%20%28single-precision%29) (DamageTypeClass :type Damage%20Type%20Class%20Reference))
  (bind _effectedactor (Variables|Default|GetEffectedActor))
  (bind _returnvalue (Transformation|GetActorLocation _effectedactor))
  (Game|Damage|ApplyPointDamage (Variables|Default|GetEffectedActor) Damage (Math|Vector|NegateVector (Transformation|GetActorForwardVector (Variables|Default|GetEffectedActor))) (Collision|MakeHitResult false false 0.0 0.0 _returnvalue _returnvalue "0,0,1" "0,0,1" 0 0) 0 (Variables|Default|GetEffectOwner) DamageTypeClass))

(fn OnEffectEnded)