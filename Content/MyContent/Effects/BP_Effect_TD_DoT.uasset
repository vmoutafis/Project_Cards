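; BP_Effect_TD_DoT is a turn-driven damage-over-time effect that hurts the effected target each turn.
; It overrides the turn start and turn end hooks, calls the parent, then applies DamagePerTurn at whichever point the ApplyDamageOn enum selects.
; SetDamagePerTurn changes the damage amount and calls EffectUpdated to signal the change.
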(fn OnTurnStart
  (|CallParentFunction)
  (if (Utilities|Enum|Equal(Enum) (Variables|Default|GetApplyDamageOn) "NewEnumerator0")
    (CallFunction|ApplyDamagetoEffected (Variables|Default|GetDamagePerTurn))))

(fn SetDamagePerTurn
  (params (Damage :type Float%20%28single-precision%29))
  (Variables|Default|SetDamagePerTurn Damage)
  (Default|CallEffectUpdated))

(fn OnTurnEnd
  (|CallParentFunction)
  (if (Utilities|Enum|Equal(Enum) (Variables|Default|GetApplyDamageOn) "NewEnumerator1")
    (CallFunction|ApplyDamagetoEffected (Variables|Default|GetDamagePerTurn))))