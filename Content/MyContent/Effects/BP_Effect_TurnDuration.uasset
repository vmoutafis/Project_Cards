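; BP_Effect_TurnDuration is an effect that lasts a set number of its affected actor's turns.
; On activation it binds to the actor's AC_TurnComponent prepare-start and prepare-end turn events, optionally firing OnTurnStart immediately, and unbinds when ended.
; Each turn end increments the completed count; EndEffectOn selects whether expiry is checked at turn start or end.
; OnTurnStart is an empty hook, and count or duration changes signal an effect update.
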(fn OnEffectActivated
  (bind _output_get (Variables|Default|SetTurnComponent (Actor|GetComponentbyClass (Variables|Default|GetEffectedActor) "/Game/MyContent/Core/AC_TurnComponent.AC_TurnComponent_C")))
  (Utilities|IsValid _output_get
    (:Is%20Valid
      (Utilities|FlowControl|Sequence
        (:then_0
          (if (Variables|Default|GetApplyEffectOnActivate)
            (CallFunction|OnTurnStart)))
        (:then_1
          (EventDispatchers|BindEventtoOnPrepareStartTurn (Variables|Default|GetTurnComponent) (EventDispatchers|CreateEvent :!event TurnStarted))
          (EventDispatchers|BindEventtoOnPrepareEndTurn (Variables|Default|GetTurnComponent) (EventDispatchers|CreateEvent :!event TurnEnded)))))))

(fn OnTurnStart)

(fn OnTurnEnd
  (if (Utilities|Enum|Equal(Enum) (Variables|Default|GetEndEffectOn) "NewEnumerator1")
    (CallFunction|TryEndEffect)))

(fn TryEndEffect
  (if (>= (Variables|Default|GetTurnsCompleted) (Variables|Default|GetTurnsDuration))
    (CallFunction|EndEffect)))

(fn TurnStarted
  (CallFunction|OnTurnStart)
  (if (Utilities|Enum|Equal(Enum) (Variables|Default|GetEndEffectOn) "NewEnumerator0")
    (CallFunction|TryEndEffect)))

(fn TurnEnded
  (CallFunction|IncrementTurnsCompleted)
  (CallFunction|OnTurnEnd)
  (if (Utilities|Enum|Equal(Enum) (Variables|Default|GetEndEffectOn) "NewEnumerator1")
    (CallFunction|TryEndEffect)))

(fn SetTurnsDuration
  (params (Duration :type Integer))
  (Variables|Default|SetTurnsDuration Duration)
  (Default|CallEffectUpdated))

(fn IncrementTurnsCompleted
  (Math|Integer|IncrementInt (Variables|Default|GetTurnsCompleted)
    (:%20%20
      (Default|CallEffectUpdated))))

(fn OnEffectEnded
  (|CallParentFunction)
  (EventDispatchers|UnbindEventfromOnPrepareStartTurn (Variables|Default|GetTurnComponent) (EventDispatchers|CreateEvent :!event TurnStarted))
  (EventDispatchers|UnbindEventfromOnPrepareEndTurn (Variables|Default|GetTurnComponent) (EventDispatchers|CreateEvent :!event TurnEnded)))