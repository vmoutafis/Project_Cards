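; Turn-based enemy for a card game that fights the player pawn with abilities and pays out currency and experience on death.
; BeginPlay scales health from a per-level multiplier table, creates its UI widget and constructs its abilities.
; On turn start it waits briefly, fires its first ability, then ends the turn when that completes.
; Damage triggers a hit-react montage, or death, which reports a loss to the TurnComponent.
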(event OnStartTurn(TurnComponent)
  (Utilities|FlowControl|Delay 2.0)
  (CallFunction|UseAbility))

(event EventBeginPlay
  (CallFunction|SetLevel (Variables|Enemy|Stats|GetLevel))
  (bind _returnvalue (UserInterface|CreateWidget "/Game/MyContent/Enemy/BP_UI_Enemy.BP_UI_Enemy_C" (Game|GetPlayerController 0)))
  (bind _output_get (Variables|Default|SetEnemyUI _returnvalue))
  (Default|InitialiseEnemyUI _output_get self)
  (UserInterface|Viewport|AddtoPlayerScreen (Variables|Default|GetEnemyUI))
  (for _array_element (Variables|Enemy|GetAbilityClasses)
    (bind _returnvalue_2 (Game|ConstructObjectfromClass self _array_element))
    (Utilities|Array|Add (Variables|Default|GetAbilitiesRef) _returnvalue_2)))

(event Game|Damage|EventAnyDamage
  (params (Damage :type Float%20%28single-precision%29) (DamageType :type Damage%20Type%20Object%20Reference) (InstigatedBy :type Controller%20Object%20Reference) (DamageCauser :type Actor%20Object%20Reference))
  (CallFunction|DamageHealth Damage))

(fn ConstructionScript
  (Variables|Default|SetHealth (Variables|Enemy|Stats|GetDefaultHealth))
  (Variables|Default|SetMaxHealth (Variables|Enemy|Stats|GetDefaultMaxHealth)))

(fn SetHealth
  (params (Health :type Float%20%28double-precision%29))
  (Variables|Default|SetHealth (Math|Float|Clamp(Float) Health 0.0 (Variables|Default|GetMaxHealth)))
  (Default|CallOnHealthChanged))

(fn SetMaxHealth
  (params (MaxHealth :type Float%20%28double-precision%29))
  (Variables|Default|SetMaxHealth (Math|Float|Max(Float) MaxHealth 0.0))
  (Default|CallOnHealthChanged))

(fn DamageHealth
  (params (Amount :type Float%20%28double-precision%29))
  (if (CallFunction|IsAlive)
    (CallFunction|SetHealth (- (Variables|Default|GetHealth) Amount))
    (Default|CallOnDamaged Amount)
    (if (not (CallFunction|IsAlive))
      (CallFunction|Death)
      (else
        (Animation|PlayAnimMontage (Variables|Enemy|GetHitReactAnim) 1.0 "None")))))

(fn IsAlive
  (return (> (Variables|Default|GetHealth) 0.0)))

(fn Death
  (Default|Lose (Variables|Default|GetTurn%20Component))
  (CallFunction|Payout)
  (Default|CallOnDeath))

(fn UseAbility
  (params (AbilityIndex :type Integer))
  (if (Utilities|Array|IsValidIndex (Variables|Default|GetAbilitiesRef) AbilityIndex)
    (bind _output_get (Variables|Default|SetActiveAbility (Utilities|Array|Get(acopy) (Variables|Default|GetAbilitiesRef) AbilityIndex)))
    (EventDispatchers|BindEventtoOnAbilityComplete _output_get (EventDispatchers|CreateEvent :!event OnAbilityComplete))
    (Default|ActivateAbility (Variables|Default|GetActiveAbility) self (Game|Player|GetPlayerPawn 0))
    (else
      (CallFunction|OnAbilityComplete))))

(fn OnAbilityComplete
  (CallFunction|ClearActiveAbility)
  (Default|SetTurnActive (Variables|Default|GetTurn%20Component) false))

(fn ClearActiveAbility
  (bind _activeability (Variables|Default|GetActiveAbility)
    (:then
      (EventDispatchers|UnbindallEventsfromOnAbilityComplete _activeability)
      (Variables|Default|SetActiveAbility 0))
    (:else)))

(fn Payout
  (Default|AddCurrency (CallFunction|GetCardGameInstance) (Variables|Enemy|GetCurrencyWorth))
  (Default|AddExperience (CallFunction|GetCardGameInstance) (Variables|Enemy|GetExperienceWorth)))

(fn SetLevel
  (params (Level :type Integer))
  (bind _returnvalue (CallFunction|GetCurrentLevelStatsMulti))
  (bind _defaultmaxhealth (Variables|Enemy|Stats|GetDefaultMaxHealth))
  (bind _returnvalue_2 (* _defaultmaxhealth (.maxhealth _returnvalue)))
  (bind _returnvalue_3 (Math|Float|Ceil _returnvalue_2))
  (Variables|Enemy|Stats|SetLevel Level)
  (CallFunction|SetMaxHealth (Math|Conversions|ToFloat(Integer) _returnvalue_3))
  (CallFunction|SetHealth (Math|Conversions|ToFloat(Integer) _returnvalue_3)))

(fn GetCurrentLevelStatsMulti
  (bind _level (Variables|Enemy|Stats|GetLevel))
  (bind _returnvalue (Math|Integer|Max(Integer) _level 1))
  (bind _returnvalue_2 (- _returnvalue 1))
  (if (Utilities|Array|IsValidIndex (Variables|Enemy|Stats|GetStatTableMultipler) _returnvalue_2)
    (return (Utilities|Array|Get(acopy) (Variables|Enemy|Stats|GetStatTableMultipler) _returnvalue_2))
    (elif (Utilities|Array|IsValidIndex (Variables|Enemy|Stats|GetStatTableMultipler) (Utilities|Array|LastIndex (Variables|Enemy|Stats|GetStatTableMultipler)))
      (return (Utilities|Array|Get(acopy) (Variables|Enemy|Stats|GetStatTableMultipler) (Utilities|Array|LastIndex (Variables|Enemy|Stats|GetStatTableMultipler))))
      (else
        (return (Utilities|Struct|MakeST_EnemyStats 0.0))))))

(fn BIBMGetTurnComponent
  (return (Variables|Default|GetTurn%20Component)))