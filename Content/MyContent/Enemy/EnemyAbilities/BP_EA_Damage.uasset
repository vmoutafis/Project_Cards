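; Enemy ability that makes the activator play a random attack montage and apply configured damage to its target.
; Damage lands on the montage's ApplyDamage notify, or on interruption, and the ability completes shortly after the montage completes or is interrupted.
; Without a valid animation, it prints a warning, applies damage immediately and completes after a delay.
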(event Custom|PlayAnimation
  (params (MontageToPlay :type Anim%20Montage%20Object%20Reference))
  (bind _notifyname (Animation|Montage|PlayMontage (Variables|/Script/Engine.Character|GetMesh (Variables|Default|GetActivator)) MontageToPlay)
    (:OnCompleted
      (CallFunction|CompleteAbilityAfterTime 0.5 :!label _label))
    (:OnInterrupted
      (Utilities|FlowControl|Sequence
        (:then_0
          (CallFunction|DoDamage :!label _label_2))
        (:then_1
          (goto _label))))
    (:OnNotifyBegin
      (if (== _notifyname "ApplyDamage")
        (goto _label_2)))))

(fn OnActivateAbility
  (if (Utilities|Array|IsEmpty (Variables|Default|GetAnimation))
    (Development|PrintString (Variables|Default|GetActivator) "No valid animation assigned to ability." :!label _label)
    (CallFunction|DoDamage)
    (CallFunction|CompleteAbilityAfterTime 1.0)
    (else
      (LocalVariables|SetLChosenAnim (.OutItem (Utilities|Array|Random (Variables|Default|GetAnimation))))
      (bind _lchosenanim (LocalVariables|GetLChosenAnim)
        (:then
          (CallFunction|PlayAnimation _lchosenanim))
        (:else
          (goto _label))))))

(fn DoDamage
  (Game|Damage|ApplyDamage (Variables|Default|GetTarget) (Variables|Default|GetDamage) 0 (Variables|Default|GetActivator) (Variables|Default|GetDamageType)))