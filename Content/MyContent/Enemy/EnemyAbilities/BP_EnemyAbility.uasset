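; BP_EnemyAbility is a generic enemy ability that can be activated on a target and reports when it completes.
; ActivateAbility stores the activator and target, then calls the OnActivateAbility hook, which by default requests completion after a short fixed delay.
; CompleteAbilityAfterTime sets a stored one-shot timer, or completes immediately for non-positive times.
; CompleteAbility fires the OnAbilityComplete dispatcher.
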(fn ActivateAbility
  (params (AbilityActivator :type BP%20Enemy%20Object%20Reference) (AbilityTarget :type Actor%20Object%20Reference))
  (Variables|Default|SetActivator AbilityActivator)
  (Variables|Default|SetTarget AbilityTarget)
  (CallFunction|OnActivateAbility)
  (return))

(fn CompleteAbility
  (Default|CallOnAbilityComplete))

(fn CompleteAbilityAfterTime
  (params (Time :type Float%20%28single-precision%29))
  (if (> Time 0.0)
    (bind _returnvalue (Utilities|Time|SetTimerbyEvent (EventDispatchers|CreateEvent :!event CompleteAbility) Time))
    (Variables|Default|SetTH_CompleteAbility _returnvalue)
    (else
      (CallFunction|CompleteAbility))))

(fn OnActivateAbility
  (CallFunction|CompleteAbilityAfterTime 1.0))