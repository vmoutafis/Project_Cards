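; Lich enemy Blueprint for turn-based combat, extending a parent enemy class with its own ability pattern and death effect.
; Each turn it increments an attack counter and uses a modulo check to pick the alternate ability every third turn.
; On death it plays a slowed timeline driving dissolve and Fresnel parameters on a dynamic mesh material created at construction, alongside the parent death logic.
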(event Custom|Dissolve
  (bind _materialinstance (Variables|Default|GetMaterialInstance))
  (Components|Timeline|SetPlayRate (Variables|Default|GetTL_Dissolve) (/ 1.0 2.0))
  (bind (_direction _dissolve _fresnel) (Timeline|TL_Dissolve PlayFromStart)
    (:Update
      (Utilities|FlowControl|Sequence
        (:then_0
          (Rendering|Material|SetScalarParameterValue _materialinstance "Dissolve" _dissolve :!class /Script/Engine.MaterialInstanceDynamic))
        (:then_1
          (Rendering|Material|SetScalarParameterValue _materialinstance "Fresnel_Exponent" _fresnel :!class /Script/Engine.MaterialInstanceDynamic))))))

(fn ConstructionScript
  (|CallParentFunction)
  (bind _returnvalue (Rendering|Material|CreateDynamicMaterialInstance (Variables|Character|GetMesh) 0 (Rendering|Material|GetMaterial (Variables|Character|GetMesh) 0) "None" :!class /Script/Engine.PrimitiveComponent))
  (Variables|Default|SetMaterialInstance _returnvalue))

(fn Death
  (CallFunction|Dissolve)
  (|CallParentFunction))

(fn BeginTurn
  (bind _result (Math|Integer|IncrementInt (Variables|Default|GetAttacksCount))
    (:%20%20
      (CallFunction|UseAbility (Math|Integer|SelectInt 1 0 (== (Math|Integer|%(Integer) _result 3) 0))))))