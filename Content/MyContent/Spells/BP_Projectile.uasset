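; Projectile spell actor that flies toward where it faces and damages its target through the owning BP_Card.
; ActivateSpell stores the target and sets ProjectileMovement velocity from the forward vector and Speed, with no steering in this graph.
; The sphere overlap destroys the projectile only when it touches that target.
; Damage is applied from the destroyed handler, passing the projectile's location and direction as hit info.
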(event OnComponentBeginOverlap(Sphere)
  (params (OverlappedComponent :type Primitive%20Component%20Object%20Reference) (OtherActor :type Actor%20Object%20Reference) (OtherComp :type Primitive%20Component%20Object%20Reference) (OtherBodyIndex :type Integer) (bFromSweep :type Boolean) (SweepResult :type Hit%20Result%20Structure%20%28by%20ref%29))
  (bind _target (Variables|Default|GetTarget)
    (:then
      (if (== _target OtherActor)
        (Actor|DestroyActor)))
    (:else)))

(event EventBeginPlay
  (Game|BindEventtoOnDestroyed (EventDispatchers|CreateEvent :!event OnProjectileDestroyed)))

(fn ConstructionScript
  (|CallParentFunction))

(fn OnProjectileDestroyed
  (params (DestroyedActor :type Actor%20Object%20Reference))
  (CallFunction|ApplyProjectileDamage))

(fn ActivateSpell
  (params (Target :type Actor%20Object%20Reference))
  (|CallParentFunction Target)
  (Variables|Default|SetTarget Target)
  (CallFunction|LaunchProjectile))

(fn LaunchProjectile
  (Variables|/Script/Engine.MovementComponent|SetVelocity (Variables|Default|GetProjectileMovement) (* (Transformation|GetActorForwardVector) (Variables|Default|GetSpeed))))

(fn ApplyProjectileDamage
  (bind _returnvalue (Transformation|GetActorLocation))
  (bind _asbp_card (Utilities|Casting|CastToBP_Card (Components|GetOwner)))
  (Default|ApplyDamagetoTarget _asbp_card (Variables|Default|GetTarget) (Transformation|GetActorForwardVector) (Collision|MakeHitResult false false 0.0 0.0 _returnvalue _returnvalue "0,0,1" "0,0,1" 0 0)))