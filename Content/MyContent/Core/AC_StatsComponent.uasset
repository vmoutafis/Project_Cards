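; Stats component that holds health, energy, armour and an alive flag for its owner.
; Setters clamp values and fire change events, while damage, heal, energy, armour and reset helpers route through them.
; Damage applies only while alive and drains armour before health; Die clears the flag and fires OnDeath.
; SetMaxEnergy passes the capped energy value to SetHealth rather than SetEnergy.
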(fn SetHealth
  (params (Health :type Float%20%28double-precision%29))
  (bind _output_get (Variables|Default|SetHealth (Math|Float|Clamp(Float) Health 0.0 (Variables|Default|GetMaxHealth))))
  (Default|CallOnHealthChanged _output_get (Variables|Default|GetMaxHealth)))

(fn SetMaxHealth
  (params (MaxHealth :type Float%20%28double-precision%29))
  (bind _output_get (Variables|Default|SetMaxHealth MaxHealth))
  (CallFunction|SetHealth (Math|Float|Min(Float) _output_get (Variables|Default|GetHealth))))

(fn SetEnergy
  (params (Energy :type Float%20%28double-precision%29))
  (bind _output_get (Variables|Default|SetEnergy (Math|Float|Clamp(Float) Energy 0.0 (Variables|Default|GetMaxEnergy))))
  (Default|CallOnEnergyChanged _output_get (Variables|Default|GetMaxEnergy)))

(fn SetMaxEnergy
  (params (MaxEnergy :type Float%20%28double-precision%29))
  (bind _output_get (Variables|Default|SetMaxEnergy MaxEnergy))
  (CallFunction|SetHealth (Math|Float|Min(Float) _output_get (Variables|Default|GetEnergy))))

(fn ApplyDamage
  (params (Damage :type Float%20%28double-precision%29))
  (LocalVariables|SetLDamageDelta (Math|Float|Max(Float) Damage 0.0))
  (if (Variables|Default|GetIsAlive)
    (Utilities|FlowControl|Sequence
      (:then_0
        (if (> (Variables|Default|GetArmour) 0.0)
          (bind _armourremoved (CallFunction|RemoveArmour (LocalVariables|GetLDamageDelta)))
          (LocalVariables|SetLDamageDelta (- (LocalVariables|GetLDamageDelta) _armourremoved))))
      (:then_1
        (if (> (LocalVariables|GetLDamageDelta) 0.0)
          (CallFunction|SetHealth (Math|Float|Clamp(Float) (- (Variables|Default|GetHealth) (LocalVariables|GetLDamageDelta)) 0.0 (Variables|Default|GetHealth)))
          (if (not (Variables|Default|GetIsAlive))
            (CallFunction|Die)))))))

(fn UseEnergy
  (params (Energy :type Float%20%28double-precision%29))
  (CallFunction|SetEnergy (Math|Float|Clamp(Float) (- (Variables|Default|GetEnergy) (Math|Float|Max(Float) Energy 0.0)) 0.0 (Variables|Default|GetEnergy))))

(fn Heal
  (params (Health :type Float%20%28double-precision%29))
  (CallFunction|SetHealth (Math|Float|Clamp(Float) (+ (Variables|Default|GetHealth) (Math|Float|Max(Float) Health 0.0)) 0.0 (Variables|Default|GetMaxHealth))))

(fn Die
  (Variables|Default|SetIsAlive false)
  (Default|CallOnDeath))

(fn Reset
  (Variables|Default|SetIsAlive true)
  (CallFunction|ResetHealth)
  (CallFunction|ResetEnergy))

(fn AddEnergy
  (params (Energy :type Float%20%28double-precision%29))
  (CallFunction|SetEnergy (+ (Variables|Default|GetEnergy) (Math|Float|Max(Float) Energy 0.0))))

(fn ResetEnergy
  (CallFunction|SetEnergy (Variables|Default|GetMaxEnergy)))

(fn ResetHealth
  (CallFunction|SetHealth (Variables|Default|GetMaxHealth)))

(fn AddArmour
  (params (Amount :type Float%20%28double-precision%29))
  (CallFunction|SetArmour (Math|Float|Max(Float) (+ (Variables|Default|GetArmour) Amount) 0.0)))

(fn SetArmour
  (params (Armour :type Float%20%28double-precision%29))
  (bind _output_get (Variables|Default|SetArmour (Math|Float|Max(Float) Armour 0.0)))
  (Default|CallOnArmourChanged _output_get))

(fn RemoveArmour
  (params (Amount :type Float%20%28double-precision%29))
  (LocalVariables|SetLArmourRemoved (Math|Float|Min(Float) Amount (Variables|Default|GetArmour)))
  (CallFunction|SetArmour (Math|Float|Max(Float) (- (Variables|Default|GetArmour) Amount) 0.0))
  (return (LocalVariables|GetLArmourRemoved)))