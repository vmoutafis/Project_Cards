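; AC_TurnComponent is an actor component that tracks whether its owner's turn is active in a battle and relays turn, win and lose events.
; SetTurnActive does nothing once the battle game mode reports completion; otherwise it stores the flag and fires start or end turn events.
; On turn start, it casts the owner to player pawn or enemy so the game mode animates the matching turn banner, including the enemy's name.
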(fn SetTurnActive
  (params (IsTurnActive :type Boolean))
  (if (not (Default|IsBattleComplete (CallFunction|GetBattleGameMode)))
    (bind _output_get (Variables|Default|SetIsTurnActive IsTurnActive))
    (if _output_get
      (Default|CallOnStartTurn)
      (Utilities|Casting|CastToBP_PlayerPawn (Components|GetOwner)
        (:then
          (Default|PlayTurnTextAnim (CallFunction|GetBattleGameMode) "PLAYER TURN"))
        (:CastFailed
          (bind _asbp_enemy (Utilities|Casting|CastToBP_Enemy (Components|GetOwner)))
          (Default|PlayTurnTextAnim (CallFunction|GetBattleGameMode) (Utilities|Text|FormatText "{name}'S TURN" (Variables|/Game/MyContent/Enemy/BP_Enemy.BP_Enemy_C|GetName _asbp_enemy)))))
      (else
        (Default|CallOnEndTurn)))))

(fn GetIsTurnActive
  (return (Variables|Default|GetIsTurnActive)))

(fn Lose
  (Default|CallOnLose self))

(fn Win
  (Default|CallOnWin))