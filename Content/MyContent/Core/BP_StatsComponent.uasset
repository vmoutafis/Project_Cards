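; BP_StatsComponent manages a character's health, energy and armour as secondary attributes, with functions for damage, healing, energy use and death.
; Setters write through SetSecondaryAttribute, capping health and energy at their maximums, then fire change events.
; ApplyDamage drains armour first, passes the remainder to health, broadcasts damage events with hit location and calls Die when health runs out.
; Reset is empty, its ResetHealth and ResetEnergy calls left unconnected.
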(fn SetHealth
  (params (Health :type Integer) (increment :type Boolean))
  (bind _returnvalue (Class|CZStatsComponent|GetSecondaryAttribute "SA_MaxHealth"))
  (bind _returnvalue_2 (Class|CZStatsComponent|SetSecondaryAttribute "SA_Health" Health increment _returnvalue))
  (Default|CallOnHealthChanged _returnvalue_2 _returnvalue))

(fn SetMaxHealth
  (params (MaxHealth :type Integer))
  (Class|CZStatsComponent|SetSecondaryAttribute "SA_MaxHealth" MaxHealth false -1)
  (CallFunction|SetHealth (Math|Integer|Min(Integer) (Class|CZStatsComponent|GetSecondaryAttribute "SA_MaxHealth") (Class|CZStatsComponent|GetSecondaryAttribute "SA_Health")) false))

(fn SetEnergy
  (params (Energy :type Integer) (increment :type Boolean))
  (bind _returnvalue (Class|CZStatsComponent|GetSecondaryAttribute "SA_MaxEnergy"))
  (bind _returnvalue_2 (Class|CZStatsComponent|SetSecondaryAttribute "SA_Energy" Energy increment _returnvalue))
  (Default|CallOnEnergyChanged _returnvalue_2 _returnvalue))

(fn SetMaxEnergy
  (params (MaxEnergy :type Integer))
  (Class|CZStatsComponent|SetSecondaryAttribute "SA_MaxEnergy" MaxEnergy false -1)
  (CallFunction|SetEnergy (Math|Integer|Min(Integer) (Class|CZStatsComponent|GetSecondaryAttribute "SA_MaxEnergy") (Class|CZStatsComponent|GetSecondaryAttribute "SA_Energy")) false))

(fn ApplyDamage
  (params (Damage :type Integer) (HitLocation :type Vector))
  (LocalVariables|SetLDamageDelta (Math|Integer|Max(Integer) Damage))
  (if (CallFunction|IsAlive)
    (Utilities|FlowControl|Sequence
      (:then_0
        (if (> (Class|CZStatsComponent|GetSecondaryAttribute "SA_Armour") 0)
          (bind _armourremoved (CallFunction|RemoveArmour (LocalVariables|GetLDamageDelta)))
          (LocalVariables|SetLArmourRemoved _armourremoved)
          (LocalVariables|SetLDamageDelta (- (LocalVariables|GetLDamageDelta) _armourremoved))
          (Default|CallOnArmourDamaged (LocalVariables|GetLArmourRemoved))
          (Default|CallOnAnyDamage (LocalVariables|GetLArmourRemoved) HitLocation)))
      (:then_1
        (if (> (LocalVariables|GetLDamageDelta) 0)
          (CallFunction|SetHealth (* (LocalVariables|GetLDamageDelta) -1) true)
          (Default|CallOnHealthDamaged (LocalVariables|GetLDamageDelta))
          (Default|CallOnAnyDamage (LocalVariables|GetLDamageDelta) HitLocation)
          (if (not (CallFunction|IsAlive))
            (CallFunction|Die)))))))

(fn UseEnergy
  (params (Energy :type Integer))
  (CallFunction|SetEnergy (Math|Integer|Clamp(Integer) (- (Class|CZStatsComponent|GetSecondaryAttribute "SA_Energy") (Math|Integer|Max(Integer) Energy)) 0 (Class|CZStatsComponent|GetSecondaryAttribute "SA_Energy")) false))

(fn Heal
  (params (Health :type Integer))
  (CallFunction|SetHealth (+ (Class|CZStatsComponent|GetSecondaryAttribute "SA_Health") (Math|Integer|Max(Integer) Health)) false))

(fn Die
  (Default|CallOnDeath))

(fn Reset)

(fn AddEnergy
  (params (Energy :type Integer))
  (CallFunction|SetEnergy Energy true))

(fn ResetEnergy
  (CallFunction|SetEnergy (Class|CZStatsComponent|GetSecondaryAttribute "SA_MaxEnergy") false))

(fn ResetHealth
  (CallFunction|SetHealth (Class|CZStatsComponent|GetSecondaryAttribute "SA_MaxHealth") false))

(fn AddArmour
  (params (Amount :type Integer))
  (CallFunction|SetArmour Amount true))

(fn SetArmour
  (params (Armour :type Integer) (increment :type Boolean))
  (bind _returnvalue (Class|CZStatsComponent|SetSecondaryAttribute "SA_Armour" Armour increment -1))
  (Default|CallOnArmourChanged _returnvalue))

(fn RemoveArmour
  (params (Amount :type Integer))
  (bind _output_get (LocalVariables|SetLArmourRemoved (Math|Integer|Min(Integer) Amount (Class|CZStatsComponent|GetSecondaryAttribute "SA_Armour"))))
  (CallFunction|SetArmour (* _output_get -1) true)
  (return (LocalVariables|GetLArmourRemoved)))

(fn IsAlive
  (return (> (Class|CZStatsComponent|GetSecondaryAttribute "SA_Health") 0)))

(fn BrodcastHealth
  (Default|CallOnHealthChanged (Class|CZStatsComponent|GetSecondaryAttribute "SA_Health") (Class|CZStatsComponent|GetSecondaryAttribute "SA_MaxHealth")))