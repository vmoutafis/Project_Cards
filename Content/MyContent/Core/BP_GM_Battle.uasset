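; Game mode for turn-based card battles that spawns the enemy stored in the game instance and creates the battle UI.
; Turn components are gathered from BI_BattleMember actors, sorted fastest first and activated cyclically, with auto-end for non-player members.
; Losing members are removed until one remains, which wins.
; A win or loss text animation then times the CompleteBattle call on the game instance.
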(event EventBeginPlay
  (Input|SetInputModeGameandUI (Game|GetPlayerController 0) 0 "DoNotLock" false false)
  (Utilities|FlowControl|Sequence
    (:then_0
      (bind _asbp_game_instance (Utilities|Casting|CastToBP_GameInstance (Game|GetGameInstance)))
      (bind _returnvalue (Actor|GetActorOfClass "/Game/MyContent/Enemy/BP_EnemySpawn.BP_EnemySpawn_C"))
      (Utilities|IsValid _returnvalue
        (:Is%20Valid
          (Game|SpawnActorfromClass (.enemy (Variables|/Game/MyContent/Core/BP_GameInstance.BP_GameInstance_C|GetEnemy _asbp_game_instance)) (Transformation|GetActorTransform _returnvalue) "Undefined" "MultiplyWithRoot" 0 (.level (Variables|/Game/MyContent/Core/BP_GameInstance.BP_GameInstance_C|GetEnemy _asbp_game_instance)) 0))))
    (:then_1
      (CallFunction|CreateUI)
      (bind _outactors (Actor|GetAllActorswithInterface "/Game/MyContent/Core/BI_BattleMember.BI_BattleMember_C"))
      (for _array_element _outactors
        (bind _returnvalue_2 (Class|BIBattleMember|BIBMGetTurnComponent(Message) _array_element))
        (Utilities|IsValid _returnvalue_2
          (:Is%20Valid
            (CallFunction|AddTurnComponent _returnvalue_2))))
      (CallFunction|StartBattle))))

(fn ConstructionScript)

(fn StartBattle
  (if (Utilities|Array|IsNotEmpty (Variables|Default|GetTurnComponents))
    (Variables|Default|SetActiveMemberIndex 0)
    (CallFunction|ToggleTurnActiveMember true)))

(fn AddTurnComponent
  (params (Component :type BP%20Turn%20Component%20Object%20Reference))
  (EventDispatchers|BindEventtoOnEndTurn Component (EventDispatchers|CreateEvent :!event OnEndTurn))
  (EventDispatchers|BindEventtoOnLose Component (EventDispatchers|CreateEvent :!event OnMemberLost))
  (for (_array_element _array_index) (Variables|Default|GetTurnComponents)
    (if (>= (Variables|/Game/MyContent/Core/BP_TurnComponent.BP_TurnComponent_C|GetTurnSpeed Component) (Variables|/Game/MyContent/Core/BP_TurnComponent.BP_TurnComponent_C|GetTurnSpeed _array_element))
      (Utilities|Array|Insert (Variables|Default|GetTurnComponents) Component _array_index)
      (return)))
  (Utilities|Array|Add (Variables|Default|GetTurnComponents) Component))

(fn OnEndTurn
  (CallFunction|ActivateNextMember))

(fn ToggleTurnActiveMember
  (params (IsTurnActive :type Boolean))
  (bind _activememberindex (Variables|Default|GetActiveMemberIndex))
  (bind _turncomponents (Variables|Default|GetTurnComponents))
  (bind _output (Utilities|Array|Get(acopy) _turncomponents _activememberindex))
  (Utilities|IsValid _output
    (:Is%20Valid
      (Default|SetTurnActive _output IsTurnActive (not (Class|CZFunctionLibrary|IsObjectOfClass (Components|GetOwner _output) "/Script/Project_Cards.CZPlayerPawn"))))
    (:Is%20Not%20Valid
      (Development|PrintString "No valid turn component." true true "(R=1.000000,G=0.000000,B=0.000000,A=1.000000)" 5.0))))

(fn IncrementActiveMemberIndex
  (bind _result (Math|Integer|IncrementInt (Variables|Default|GetActiveMemberIndex))
    (:%20%20
      (if (> _result (Utilities|Array|LastIndex (Variables|Default|GetTurnComponents)))
        (Variables|Default|SetActiveMemberIndex 0)))))

(fn ActivateNextMember
  (CallFunction|IncrementActiveMemberIndex)
  (CallFunction|ToggleTurnActiveMember true))

(fn CreateUI
  (bind _returnvalue (UserInterface|CreateWidget "/Game/MyContent/Core/UI/BP_UI_BattleMode.BP_UI_BattleMode_C" (Game|GetPlayerController 0)))
  (bind _output_get (Variables|Default|SetBattleModeUI _returnvalue))
  (UserInterface|Viewport|AddtoPlayerScreen _output_get))

(fn PlayTurnTextAnim
  (params (Text :type Text))
  (bind _battlemodeui (Variables|Default|GetBattleModeUI)
    (:then
      (bind _duration (Default|PlayTurnText _battlemodeui Text))
      (return _duration))
    (:else
      (return 0.0))))

(fn OnMemberLost
  (params (Component :type BP%20Turn%20Component%20Object%20Reference))
  (bind _turncomponents (Variables|Default|GetTurnComponents))
  (bind _output (Utilities|Array|Get(acopy) _turncomponents))
  (Utilities|Array|RemoveItem (Variables|Default|GetTurnComponents) Component)
  (if (CallFunction|IsBattleComplete)
    (Default|Win _output)
    (Utilities|Casting|CastToBP_CardsPawn (Components|GetOwner _output)
      (:then
        (bind _duration (CallFunction|PlayWinTextAnim "BATTLE WON"))
        (Utilities|Time|SetTimerbyEvent (EventDispatchers|CreateEvent :!event WinBattle) _duration))
      (:CastFailed
        (bind _duration_2 (CallFunction|PlayTurnTextAnim "BATTLE LOST"))
        (Utilities|Time|SetTimerbyEvent (EventDispatchers|CreateEvent :!event LoseBattle) _duration_2)))))

(fn PlayWinTextAnim
  (params (Text :type Text))
  (bind _battlemodeui (Variables|Default|GetBattleModeUI)
    (:then
      (bind _duration (Default|PlayWinGameText _battlemodeui Text))
      (return _duration))
    (:else
      (return 0.0))))

(fn WinBattle
  (bind _asbp_game_instance (Utilities|Casting|CastToBP_GameInstance (Game|GetGameInstance)))
  (Default|CompleteBattle _asbp_game_instance true))

(fn LoseBattle
  (Default|CompleteBattle (CallFunction|GetCardGameInstance) false))

(fn IsBattleComplete
  (return (< (Utilities|Array|Length (Variables|Default|GetTurnComponents)) 2)))