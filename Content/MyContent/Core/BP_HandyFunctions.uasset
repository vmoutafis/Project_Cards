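; Blueprint helper library for the card game, with shortcuts to the game instance and battle game mode plus a card description builder.
; CreateCardDescription reads a card class's defaults through per-stat steps for damage, healing, armour, critical strike, double hit and effects (Bleed, Burn, Shock).
; Each step appends a data table text row, replacing placeholder tokens with values; damage and healing include game instance attributes.
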(fn GetCardGameInstance
  (return (.AsBP%20Game%20Instance (Utilities|Casting|CastToBP_GameInstance (Game|GetGameInstance (LocalVariables|Get__WorldContext))))))

(fn GetBattleGameMode
  (bind _asbp_gm_battle (Utilities|Casting|CastToBP_GM_Battle (Game|GetGameMode (LocalVariables|Get__WorldContext))))
  (return _asbp_gm_battle))

(fn CreateCardDescription
  (params (Card :type BP%20Card%20Class%20Reference))
  (|Damage)
  (|Healing)
  (|Armour)
  (|CriticalStrike)
  (|DoubleHit)
  (|Effects)
  (return (LocalVariables|GetLFinalDescription)))